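; Asteroid spawner that continuously spawns BP_Astroid actors in a donut-shaped area around the player pawn.
; From BeginPlay, an endless loop spawns one asteroid, waits SpawnDelay, then repeats.
; Each location uses a random yaw, the player's pitch and roll, and a random distance between MinimumSpawnRange and MaximumSpawnRange.
; Spawn yaw comes from a look-at rotation toward the player, aiming asteroids inward.
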(event `self.ReceiveBeginPlay`
  (bind _returnvalue (`GameplayStatics.GetPlayerPawn` 0))
  (bind (_returnvalue_roll _returnvalue_pitch) (`KismetMathLibrary.BreakRotator` (`self.K2_GetActorRotation` _returnvalue)))
  (bind _returnvalue_2 (+ (`self.K2_GetActorLocation` _returnvalue) (* (`KismetMathLibrary.Conv_RotatorToVector` (`KismetMathLibrary.MakeRotator` _returnvalue_roll _returnvalue_pitch (`KismetMathLibrary.RandomFloatInRange` 0.0 360.0))) (`KismetMathLibrary.RandomFloatInRange` (`self.MinimumSpawnRange`) (`self.MaximumSpawnRange`)))))
  (bind (_returnvalue_roll_2 _returnvalue_pitch_2 _returnvalue_yaw) (`KismetMathLibrary.BreakRotator` (`KismetMathLibrary.FindLookAtRotation` _returnvalue_2 (`self.K2_GetActorLocation` (`GameplayStatics.GetPlayerPawn` 0)))))
  (`|SpawnActorFromClass` "/Game/Alan/BP_Astroid.BP_Astroid_C" (`KismetMathLibrary.MakeTransform` _returnvalue_2 (`KismetMathLibrary.MakeRotator` 0.0 0.0 _returnvalue_yaw)) "Undefined" "MultiplyWithRoot" null null :!label _label)
  (`KismetSystemLibrary.Delay` (`self.SpawnDelay`))
  (goto _label))

(fn `UserConstructionScript`)