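; BP_AstroidM is a clickable asteroid actor that blows up when the player clicks it.
; BeginPlay enables click events on the first player controller so the Sphere component receives clicks.
; A click waits briefly, then destroys the actor and spawns a scaled-up explosion emitter and sound at its location.
; An Explode flag gates the click, though it is only set at the end of that sequence.
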(event `self.ReceiveBeginPlay`
  (set `PlayerController.bEnableClickEvents` true (`GameplayStatics.GetPlayerController` 0)))

(event `self.Sphere.OnClicked`
  (params (TouchedComponent :type "PrimitiveComponent Object Reference") (ButtonPressed :type "Key Structure"))
  (bind _returnvalue (`self.K2_GetActorLocation`))
  (if (not (`self.Explode`))
    (`KismetSystemLibrary.Delay` 0.2)
    (`self.K2_DestroyActor`)
    (`GameplayStatics.SpawnEmitterAtLocation` "/Game/StarterContent/Particles/P_Explosion.P_Explosion" _returnvalue (struct) (2.0 2.0 2.0))
    (`GameplayStatics.PlaySoundAtLocation` "/Game/StarterContent/Audio/Explosion01.Explosion01" _returnvalue (struct) 1.0 1.0 0.0 null null null null)
    (set `self.Explode` true)))

(fn `UserConstructionScript`)